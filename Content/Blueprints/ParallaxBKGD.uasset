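; ParallaxBKGD is a background actor meant to scroll horizontally for parallax in a 2D side-scroller.
; Each Tick it reads the side-scroller character's moving-right and moving-left flags and offsets itself along X against that direction, scaled by ParallaxSpeed.
; As written, the offset multiplies the length of a zero vector, so it is always zero.
; The cast supplying the character reference is never executed.
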(event EventTick
  (params (DeltaSeconds :type Float%20%28single-precision%29))
  (bind _returnvalue (Transformation|GetActorLocation))
  (bind _returnvalue_2 (Math|Vector|VectorLength "0, 0, 0"))
  (bind _parallaxspeed (Variables|Default|GetParallaxSpeed))
  (bind _returnvalue_3 (* _returnvalue_2 _parallaxspeed))
  (bind _returnvalue_4 (Math|Vector|MakeVector _returnvalue_3 0.0 0.0))
  (if (Variables|/Game/2DSideScrollerBP/Blueprints/2DSideScrollerCharacter.2DSideScrollerCharacter_C|GetbisMovingRight (stale _as2dside_scroller_character))
    (Transformation|SetActorRelativeLocation (- _returnvalue _returnvalue_4))
    (elif (Variables|/Game/2DSideScrollerBP/Blueprints/2DSideScrollerCharacter.2DSideScrollerCharacter_C|Getmovingleft (stale _as2dside_scroller_character))
      (Transformation|SetActorRelativeLocation (+ _returnvalue _returnvalue_4)))))

(fn ConstructionScript)